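; Showcase trigger actor meant to open a talent tree window when a Pawn enters its capsule.
; A valid, hidden TalentTreeWindow is added to the player screen; otherwise a UMG_Skill_Tree widget is created for player 0 but never stored or shown.
; Disconnected logic would call TriggerWindow on PrototypeUI_Controller with TriggerName, deactivate PTrigger once, and clear the window reference.
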(event `self.Capsule.OnComponentBeginOverlap`
  (params (OverlappedComponent :type "PrimitiveComponent Object Reference") (OtherActor :type "Actor Object Reference") (OtherComp :type "PrimitiveComponent Object Reference") (OtherBodyIndex :type Integer) (bFromSweep :type Boolean) (SweepResult :type "HitResult Structure (by ref)"))
  (bind _talent_tree_window (`self.Talent Tree Window`))
  (cast `Pawn` OtherActor)
  ;[0.32 0.007392 0] Talent Tree
  (`/Engine/EditorBlueprintResources/StandardMacros.IsValid` (`self.Talent Tree Window`)
    (:`Is Valid`
      (if (not (`Widget.IsInViewport` _talent_tree_window))
        (`UserWidget.AddToPlayerScreen` _talent_tree_window 0)))
    (:`Is Not Valid`
      (bind _returnvalue (`|CreateWidget` "/Game/Assimilate/UI/SkillTree/UMG_Skill_Tree.UMG_Skill_Tree_C" (`GameplayStatics.GetPlayerController` 0))))))

(fn `UserConstructionScript`)