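; Level manager for Assimilate that plays the level song, shows mission text and moves the game to the next level.
; On BeginPlay it caches the W_ScreenGame widget after a short delay, then shows the start text, which StartMission can also trigger.
; EndMission shows the end text, waits, then opens NextLevel by name.
; A camera fade sequence is present but unconnected.
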(event `self.ReceiveBeginPlay`
  (`|ExecutionSequence`
    (:`then_0`
      (`GameplayStatics.PlaySound2D` (`self.LevelSong`) 1.0 1.0 0.0 null null))
    (:`then_1`
      (`KismetSystemLibrary.Delay` 0.2)
      (bind _foundwidgets (`WidgetBlueprintLibrary.GetAllWidgetsOfClass` "/Game/Assimilate/UI/W_ScreenGame.W_ScreenGame_C"))
      (for _array_element _foundwidgets
        (set `self.ScreenGame` _array_element)))
    (:`then_2`
      (`KismetSystemLibrary.Delay` 1.0)
      (`/Game/Assimilate/UI/W_ScreenGame.MiddleText` (`self.ScreenGame`) (`self.StartMissionText`) :!label _label))))

(event `StartMission`
  (params (MiddleText1 :type String))
  (goto _label))

(event `EndMission`
  (`/Game/Assimilate/UI/W_ScreenGame.MiddleText` (`self.ScreenGame`) (`self.EndMissionOneText`))
  (`KismetSystemLibrary.Delay` 8.0)
  (`GameplayStatics.OpenLevel` (`self.NextLevel`)))

(fn `UserConstructionScript`)