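; Resource pickup actor that adds 5 resources to the Assimilate game state and destroys itself when a BP_ThousandEagle overlaps its Sphere.
; An outer SphereOutbox acts as a magnet: on player pawn overlap, MoveComponentTo pulls the root to the pawn's location, then snaps it there again after a delay.
; A ship health bonus exists in the graph but is disconnected and never runs.
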(event `self.Sphere.OnComponentBeginOverlap`
  (params (OverlappedComponent :type "PrimitiveComponent Object Reference") (OtherActor :type "Actor Object Reference") (OtherComp :type "PrimitiveComponent Object Reference") (OtherBodyIndex :type Integer) (bFromSweep :type Boolean) (SweepResult :type "HitResult Structure (by ref)"))
  (bind _asbp_thousand_eagle (cast `/Game/Assimilate/Character/Pawn/BP_ThousandEagle` OtherActor))
  (`/Game/Assimilate/Core/AssimilateGameStateBase.AddRessources` (`/Game/Assimilate/Core/AssimilateFunctionLibrary.GameStateAssimilate`) 5)
  (`self.K2_DestroyActor`))

(event `self.SphereOutbox.OnComponentBeginOverlap`
  (params (OverlappedComponent :type "PrimitiveComponent Object Reference") (OtherActor :type "Actor Object Reference") (OtherComp :type "PrimitiveComponent Object Reference") (OtherBodyIndex :type Integer) (bFromSweep :type Boolean) (SweepResult :type "HitResult Structure (by ref)"))
  (if (== OtherActor (`GameplayStatics.GetPlayerPawn` 0))
    (`KismetSystemLibrary.MoveComponentTo` (`self.DefaultSceneRoot`) (`self.K2_GetActorLocation` (`GameplayStatics.GetPlayerPawn` 0)) (struct) false false (`KismetMathLibrary.Lerp` 0.0 0.2 1.0))
    (`KismetSystemLibrary.Delay` 2.0)
    (`KismetSystemLibrary.MoveComponentTo` (`self.DefaultSceneRoot`) (`self.K2_GetActorLocation` (`GameplayStatics.GetPlayerPawn` 0)) (struct) false false 0.0)))

(fn `UserConstructionScript`)