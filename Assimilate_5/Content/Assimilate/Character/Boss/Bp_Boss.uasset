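; Boss actor that takes damage and ends the mission when defeated.
; Each hit taken with health left subtracts damage, prints the health and moves the root toward the first target point's location.
; Health is checked before subtracting, so a hit arriving at zero or below triggers death: explosion, cube removal, a short delay, EndMission on the level manager, then self-destruction.
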(event `self.ReceiveAnyDamage`
  (params (Damage :type "Float (single-precision)") (DamageType :type "DamageType Object Reference") (InstigatedBy :type "Controller Object Reference") (DamageCauser :type "Actor Object Reference"))
  (bind _health (`self.Health`))
  ;[1 0 0] Take Damage
  (if (<= _health 0)
    (`GameplayStatics.SpawnEmitterAtLocation` "/Game/Assimilate/Particles/P_Asteroid_Explosion.P_Asteroid_Explosion" (`SceneComponent.K2_GetComponentLocation` (`self.Cube`)) (struct) (`SceneComponent.K2_GetComponentScale` (`self.DefaultSceneRoot`)))
    (`ActorComponent.K2_DestroyComponent` (`self.Cube`))
    (`KismetSystemLibrary.Delay` 2.0)
    (bind _outactors (`GameplayStatics.GetAllActorsOfClass` "/Game/Assimilate/Blueprints/Bp_LevelManager.Bp_LevelManager_C"))
    (`/Game/Assimilate/Blueprints/Bp_LevelManager.EndMission` (`|GetArrayItem` _outactors))
    (`self.K2_DestroyActor`)
    (else
      (bind _output_get (set `self.Health` (- _health (`KismetMathLibrary.FTrunc` Damage))))
      (`KismetSystemLibrary.PrintString` (`KismetStringLibrary.Conv_IntToString` _output_get))
      (`KismetSystemLibrary.MoveComponentTo` (`self.DefaultSceneRoot`) (`self.K2_GetActorLocation` (`|GetArrayItem` (`self.TargetPoint`)))))))

(fn `UserConstructionScript`)