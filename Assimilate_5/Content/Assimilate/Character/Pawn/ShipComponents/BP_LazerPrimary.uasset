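; BP_LazerPrimary is a ship's primary laser weapon actor that spawns laser shots at its own location and rotation.
; Fire spawns a BP_LazerProjectile, plays the firing sound and attaches a particle emitter, while BeamFire only spawns a BP_LazerProjectileBeam.
; Both pass the parent ship and stored damage, speed, physics and visual settings to the spawned actor.
; LazerPropertyFunction writes most of those settings, and FirePower calls it with unset inputs.
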(event `FirePower`
  (`self.LazerPropertyFunction` 0.0))

(event `BeamFire`
  (`|SpawnActorFromClass` "/Game/Assimilate/Character/Pawn/ShipComponents/BP_LazerProjectileBeam.BP_LazerProjectileBeam_C" (`KismetMathLibrary.MakeTransform` (`self.K2_GetActorLocation`) (`self.K2_GetActorRotation`) (`KismetMathLibrary.Conv_DoubleToVector` (`self.Lazer_Primary_Scale`))) "Undefined" "OverrideRootScale" null (`self.Lazer_Primary_Color`) (`self.Lazer_Primary_PhysicsForce`) (`self.Lazer_Primary_ExplosionScale`) (`self.ParentShip`) (`self.Lazer_Primary_DamageToApply`) (`self.Lazer_Primary_PhysicsForce_Multiplier_ForShield`) (`self.Lazer_Primary_Speed`) (`self.Lazer_Primary_ExplosionBrightness`) (`self.Lazer_Primary_PointLightBrightness`) (`self.Lazer_Primary_PointLightEnabled`) (`self.Lazer_Primary_MaterialGlowIntensity`) null))

(event `Fire`
  (bind _returnvalue (`self.K2_GetActorLocation`))
  (bind _returnvalue_2 (`|SpawnActorFromClass` "/Game/Assimilate/Character/Pawn/ShipComponents/BP_LazerProjectile.BP_LazerProjectile_C" (`KismetMathLibrary.MakeTransform` _returnvalue (`self.K2_GetActorRotation`) (`KismetMathLibrary.Conv_DoubleToVector` (`self.Lazer_Primary_Scale`))) "Undefined" "OverrideRootScale" null (`self.Lazer_Primary_Color`) (`self.Lazer_Primary_PhysicsForce`) (`self.Lazer_Primary_ExplosionScale`) (`self.ParentShip`) (`self.Lazer_Primary_DamageToApply`) (`self.Lazer_Primary_PhysicsForce_Multiplier_ForShield`) (`self.Lazer_Primary_Speed`) (`self.Lazer_Primary_ExplosionBrightness`) (`self.Lazer_Primary_PointLightBrightness`) (`self.Lazer_Primary_PointLightEnabled`) (`self.Lazer_Primary_MaterialGlowIntensity`) self))
  (`GameplayStatics.PlaySoundAtLocation` (`self.Lazer_Primary_SoundCue`) _returnvalue (struct) 0.5 1.0 0.0 null null null)
  (`GameplayStatics.SpawnEmitterAttached` (`self.Particles`) (`/Game/Assimilate/Character/Pawn/ShipComponents/BP_LazerProjectile.Cylinder` _returnvalue_2) "None" (`self.K2_GetActorLocation` _returnvalue_2) (struct) (1.0 1.0 1.0) "SnapToTargetIncludingScale" false))

(fn `LazerPropertyFunction`
  (params (Lazer_Primary_Scale :type "Float (double-precision)") (Lazer_Primary_Color :type "LinearColor Structure") (Lazer_Primary_WaitDelay :type "Float (double-precision)") (Lazer_Primary_PhysicsForce_Multiplier_ForShield :type "Float (double-precision)") (Lazer_Primary_DamageToApply :type "Float (double-precision)") (Lazer_Primary_Speed :type "Float (double-precision)") (Lazer_Primary_ExplosionScale :type "Float (double-precision)") (Lazer_Primary_PointLightBrightness :type "Float (double-precision)") (Lazer_Primary_ExplosionBrightness :type "Float (double-precision)") (Lazer_Primary_PointLightEnabled :type Boolean) (Lazer_Primary_SoundCue :type "SoundBase Object Reference") (Lazer_Primary_MaterialGlowIntensity :type "Float (double-precision)"))
  (set `self.Lazer_Primary_Scale` Lazer_Primary_Scale)
  (set `self.Lazer_Primary_Color` Lazer_Primary_Color)
  (set `self.Lazer_Primary_WaitDelay` Lazer_Primary_WaitDelay)
  (set `self.Lazer_Primary_PhysicsForce_Multiplier_ForShield` Lazer_Primary_PhysicsForce_Multiplier_ForShield)
  (set `self.Lazer_Primary_DamageToApply` Lazer_Primary_DamageToApply)
  (set `self.Lazer_Primary_Speed` Lazer_Primary_Speed)
  (set `self.Lazer_Primary_ExplosionScale` Lazer_Primary_ExplosionScale)
  (set `self.Lazer_Primary_PointLightBrightness` Lazer_Primary_PointLightBrightness)
  (set `self.Lazer_Primary_ExplosionBrightness` Lazer_Primary_ExplosionBrightness)
  (set `self.Lazer_Primary_PointLightEnabled` Lazer_Primary_PointLightEnabled)
  (set `self.Lazer_Primary_SoundCue` Lazer_Primary_SoundCue)
  (set `self.Lazer_Primary_MaterialGlowIntensity` Lazer_Primary_MaterialGlowIntensity)
  (return))

(fn `UserConstructionScript`)