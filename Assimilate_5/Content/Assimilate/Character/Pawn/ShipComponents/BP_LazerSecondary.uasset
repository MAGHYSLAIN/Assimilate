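; BP_LazerSecondary is a ship's secondary laser weapon, spawning projectiles at its own transform.
; Fire launches a rapid-fire burst of BP_LazerProjectile, looping through a Delay and counter, with an optional sound per round.
; BeamFire spawns one BP_LazerProjectileSecondBeam without sound, with fixed explosion scale and no material glow.
; Both pass the weapon's damage, physics, speed and visual settings to the projectile, plus ParentShip as shooter.
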(event `BeamFire`
  (`|SpawnActorFromClass` "/Game/Assimilate/Character/Pawn/ShipComponents/BP_LazerProjectileSecondBeam.BP_LazerProjectileSecondBeam_C" (`KismetMathLibrary.MakeTransform` (`self.K2_GetActorLocation`) (`self.K2_GetActorRotation`) (`KismetMathLibrary.Conv_DoubleToVector` (`self.Lazer_Secondary_Scale`))) "Undefined" "OverrideRootScale" null (`self.Lazer_Secondary_Color`) (`self.Lazer_Secondary_PhysicsForce`) 5.0 (`self.ParentShip`) (`self.Lazer_Secondary_DamageToApply`) (`self.Lazer_Secondary_PhysicsForce_Multiplier_ForShield`) (`self.Lazer_Secondary_Speed`) (`self.Lazer_Secondary_ExplosionBrightness`) (`self.Lazer_Secondary_PointLightBrightness`) (`self.Lazer_Secondary_PointLightEnabled`) 0.0 self))

(event `Fire`
  (bind _lazer_secondary_soundcue (`self.Lazer_Secondary_SoundCue`))
  (`|SpawnActorFromClass` "/Game/Assimilate/Character/Pawn/ShipComponents/BP_LazerProjectile.BP_LazerProjectile_C" (`KismetMathLibrary.MakeTransform` (`self.K2_GetActorLocation`) (`self.K2_GetActorRotation`) (`KismetMathLibrary.Conv_DoubleToVector` (`self.Lazer_Secondary_Scale`))) "Undefined" "OverrideRootScale" null (`self.Lazer_Secondary_Color`) (`self.Lazer_Secondary_PhysicsForce`) (`self.Lazer_Secondary_Explosion Scale`) (`self.ParentShip`) (`self.Lazer_Secondary_DamageToApply`) (`self.Lazer_Secondary_PhysicsForce_Multiplier_ForShield`) (`self.Lazer_Secondary_Speed`) (`self.Lazer_Secondary_ExplosionBrightness`) (`self.Lazer_Secondary_PointLightBrightness`) (`self.Lazer_Secondary_PointLightEnabled`) (`self.Lazer_Secondary_MaterialGlowIntensity`) self :!label _label)
  (set `self.Lazer_Secondary_RapidFire_Count` (+ (`self.Lazer_Secondary_RapidFire_Count`) 1))
  (`/Engine/EditorBlueprintResources/StandardMacros.IsValid` _lazer_secondary_soundcue
    (:`Is Valid`
      (`GameplayStatics.PlaySoundAtLocation` _lazer_secondary_soundcue (`self.K2_GetActorLocation`) (struct) 1.0 1.0 0.0 null null null))
    (:`Is Not Valid`
      _))
  (`KismetSystemLibrary.Delay` (`self.Lazer_Secondary_RapidFire_Round_Delay`))
  (if (>= (`self.Lazer_Secondary_RapidFire_Count`) (`self.Lazer_Secondary_RapidFire_Rounds`))
    (set `self.Lazer_Secondary_RapidFire_Count` 0)
    (else
      (goto _label))))

(fn `UserConstructionScript`)