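; Target actor whose Widget1 component turns to face the player's BP_ThousandEagle pawn every tick.
; The rotation comes from the normalized direction between the widget and the pawn, and is skipped if the player pawn is another class.
; Five seconds after BeginPlay it caches the first top-level W_Target widget.
; SetHit and UnsetHit are empty, as the calls that change that widget's hit color are disconnected.
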(event `self.ReceiveBeginPlay`
  (`KismetSystemLibrary.Delay` 5.0)
  (bind _foundwidgets (`WidgetBlueprintLibrary.GetAllWidgetsOfClass` "/Game/Assimilate/UI/W_Target.W_Target_C"))
  (set `self.Umg_Target` (`|GetArrayItem` _foundwidgets)))

(event `SetHit`)

(event `UnsetHit`)

(event `self.ReceiveTick`
  (params (DeltaSeconds :type "Float (single-precision)"))
  (bind _asbp_thousand_eagle (cast `/Game/Assimilate/Character/Pawn/BP_ThousandEagle` (`GameplayStatics.GetPlayerPawn` 0)))
  (`SceneComponent.K2_SetWorldRotation` (`self.Widget1`) (`KismetMathLibrary.Conv_VectorToRotator` (`KismetMathLibrary.GreaterGreater_VectorRotator` (`KismetMathLibrary.Normal` (* (- (`self.K2_GetActorLocation` _asbp_thousand_eagle) (`SceneComponent.K2_GetComponentLocation` (`self.Widget1`))) (1.0 1.0 1.0))))) false false))

(fn `UserConstructionScript`)